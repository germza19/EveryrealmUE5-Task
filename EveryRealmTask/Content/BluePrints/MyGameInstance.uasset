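; Game instance Blueprint that tracks which character button is currently selected, likely for a character selection menu.
; On init it resets the character index to zero.
; Three check functions, for hover, click and unhover, compare a passed button with the stored one and return whether it is selected.
; A click on another button deselects the old one and stores the new one, with debug prints throughout.
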(event EventInit
  (bind _output_get (Variables|Default|SetCurrentCharacterIndex 0))
  (Development|PrintString (Utilities|String|ToString(Integer) _output_get)))

(fn CheckonButtonHovered
  (params (CharacterButton :type WB%20Character%20Button%20Object%20Reference))
  (if (== CharacterButton (Variables|Default|GetCurrentCharacterButton))
    (Development|PrintString "Is Selected one")
    (return true)
    (else
      (Development|PrintString "Not selected one")
      (return false))))

(fn CheckonButtonClicked
  (params (CharacterButton :type WB%20Character%20Button%20Object%20Reference))
  (if (== CharacterButton (Variables|Default|GetCurrentCharacterButton))
    (Development|PrintString "Is Selected one, do nothing")
    (return true)
    (else
      (Development|PrintString "Not selected one, Selected new One")
      (Default|OnDeselected (Variables|Default|GetCurrentCharacterButton))
      (Variables|Default|SetCurrentCharacterButton CharacterButton)
      (return false))))

(fn CheckonButtonUnhovered
  (params (CharacterButton :type WB%20Character%20Button%20Object%20Reference))
  (if (== CharacterButton (Variables|Default|GetCurrentCharacterButton))
    (Development|PrintString "Is Selected one, Do nothing")
    (return true)
    (else
      (Development|PrintString "Not selected one, play unhover")
      (return false))))